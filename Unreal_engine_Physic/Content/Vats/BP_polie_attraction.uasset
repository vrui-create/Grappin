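; BP_polie_attraction is a physics-constraint actor, apparently a pulley, that animates when the right mouse button is pressed.
; BeginPlay enables player input, and the press plays a timeline.
; Each update sets one constraint component's relative yaw and feeds the second constraint's linear position target.
; Disconnected logic remains for flipping an angular orientation target and nudging the Frame with an impulse.
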(event `Key|RightMouseButton`
  (params (Key :type "Key Structure"))
  (:`Pressed`
    (bind (_direction _set_rotator _set_location) (`Timeline|Timeline`)
      (:`Update`
        (`SceneComponent.K2_SetRelativeRotation` (`self.PhysicsConstraint`) (`KismetMathLibrary.MakeRotator` 0.0 0.0 _set_rotator) false false)
        (bind _returnvalue (`PhysicsConstraintComponent.GetConstraint` (`self.PhysicsConstraint1`)))
        (`ConstraintInstanceBlueprintLibrary.SetLinearPositionTarget` _returnvalue (`KismetMathLibrary.Conv_DoubleToVector` _set_location))))))

(event `Key|RightMouseButton`
  (params (Key :type "Key Structure")))

(event `Key|LeftMouseButton`
  (params (Key :type "Key Structure")))

(event `self.ReceiveBeginPlay`
  (`self.EnableInput` self (`GameplayStatics.GetPlayerController` 0)))

(fn `UserConstructionScript`)