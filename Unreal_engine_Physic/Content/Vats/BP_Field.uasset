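; Chaos field actor that breaks and pushes destructible geometry through an explosion event, ceexplose.
; The event applies external cluster strain with linear radial falloff sized to its Sphere, then one second later adds a radial linear force from the actor's location.
; BeginPlay starts a looping one-second timer with no event shown bound to it, and a culling field node is left unused.
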(event `self.ReceiveBeginPlay`
  (`KismetSystemLibrary.K2_SetTimerDelegate` :`Time` 1.0 :`bLooping` true))

(event `ce explose`
  (bind _sphere (`self.Sphere`))
  (`FieldSystemComponent.ApplyPhysicsField` (`self.FieldSystemComponent`) true "Field_ExternalClusterStrain" null (`RadialFalloff.SetRadialFalloff` (`self.RadialFalloff`) (`self.Field Magnitude`) 0.0 10.0 0.0 (`SphereComponent.GetScaledSphereRadius` _sphere) (`SceneComponent.K2_GetComponentLocation` _sphere) "Field_Falloff_Linear"))
  (`KismetSystemLibrary.Delay` 1.0)
  (`FieldSystemComponent.ApplyPhysicsField` (`self.FieldSystemComponent`) true "Field_LinearForce" null (`RadialVector.SetRadialVector` (`self.RadialVector`) 100.0 (`self.K2_GetActorLocation`))))

(fn `UserConstructionScript`)