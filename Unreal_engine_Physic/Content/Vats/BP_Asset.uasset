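; BP_Asset is a configurable physics prop that bounces off actors tagged Bumper.
; At BeginPlay its static mesh component receives the mesh, gravity setting, scale and mass scale from variables and starts simulating physics.
; On hitting a Bumper, the mesh gets a velocity-change impulse along the impact normal scaled by Intensity, so mass does not affect the bounce.
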(event `self.ReceiveBeginPlay`
  (bind _staticmesh (`self.StaticMesh`))
  (`PrimitiveComponent.SetEnableGravity` _staticmesh (`self.Gravity Enabled`))
  (`StaticMeshComponent.SetStaticMesh` _staticmesh (`self.Mesh`))
  (`PrimitiveComponent.SetSimulatePhysics` _staticmesh true)
  (`SceneComponent.SetRelativeScale3D` _staticmesh (`KismetMathLibrary.Conv_DoubleToVector` (`self.Scale_Taille`)))
  (`PrimitiveComponent.SetMassScale` _staticmesh "None" (`self.In Mass Scale`)))

(event `self.StaticMesh.OnComponentHit`
  (params (HitComponent :type "PrimitiveComponent Object Reference") (OtherActor :type "Actor Object Reference") (OtherComp :type "PrimitiveComponent Object Reference") (NormalImpulse :type "Vector Structure") (Hit :type "HitResult Structure (by ref)"))
  (if (`self.ActorHasTag` OtherActor "Bumper")
    (`PrimitiveComponent.AddImpulse` (`self.StaticMesh`) (* (`.ImpactNormal` (`GameplayStatics.BreakHitResult` Hit)) (`KismetMathLibrary.Conv_DoubleToVector` (`self.Intensity`))) "None" true)))

(fn `UserConstructionScript`)