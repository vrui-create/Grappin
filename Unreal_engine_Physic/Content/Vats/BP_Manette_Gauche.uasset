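; BP_Manette_Gauche is a physics-driven interactable, apparently a left lever, that the player swings between two angles with mouse clicks.
; Overlapping its Sphere enables input and shows the HUD interaction prompt for the cached third-person character; leaving reverses both.
; Left and right clicks flip the PhysicsConstraint's angular orientation target to opposite sides, then apply a tiny impulse to Frame.
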(event `Key|RightMouseButton`
  (params (Key :type "Key Structure"))
  (:`Pressed`
    (`KismetSystemLibrary.PrintString` "R")
    (set `self.bool_Angulaire` false)
    (bind _returnvalue (`PhysicsConstraintComponent.GetConstraint` (`self.PhysicsConstraint`) :!label _label))
    (`ConstraintInstanceBlueprintLibrary.SetAngularOrientationTarget` _returnvalue (select `bool` (`self.bool_Angulaire`) :`false` (`KismetMathLibrary.MakeRotator` 0.0 0.0 80.0) :`true` (`KismetMathLibrary.MakeRotator` 0.0 0.0 -80.0) :!type "Rotator Structure"))
    (`PrimitiveComponent.AddImpulse` (`self.Frame`) (0.1 0.1 0.1) "None" true)))

(event `Key|LeftMouseButton`
  (params (Key :type "Key Structure"))
  (:`Pressed`
    (`KismetSystemLibrary.PrintString` "L")
    (set `self.bool_Angulaire` true)
    (goto _label)))

(event `self.ReceiveBeginPlay`
  (bind _asbp_third_person_character (cast `/Game/ThirdPerson/Blueprints/BP_ThirdPersonCharacter` (`GameplayStatics.GetPlayerCharacter` 0)))
  (set `self.REF_Player` _asbp_third_person_character))

(event `self.Sphere.OnComponentBeginOverlap`
  (params (OverlappedComponent :type "PrimitiveComponent Object Reference") (OtherActor :type "Actor Object Reference") (OtherComp :type "PrimitiveComponent Object Reference") (OtherBodyIndex :type Integer) (bFromSweep :type Boolean) (SweepResult :type "HitResult Structure (by ref)"))
  (`self.M_Cardre player Interaction` true OtherActor))

(event `self.Sphere.OnComponentEndOverlap`
  (params (OverlappedComponent :type "PrimitiveComponent Object Reference") (OtherActor :type "Actor Object Reference") (OtherComp :type "PrimitiveComponent Object Reference") (OtherBodyIndex :type Integer))
  (`self.M_Cardre player Interaction` false OtherActor))

(fn `UserConstructionScript`)