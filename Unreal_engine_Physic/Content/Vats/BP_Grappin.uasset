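; BP_Grappin is a grappling hook projectile that pulls the player toward whatever it hits.
; Its cable end attaches to the player's head; on hit, the actor attaches to the target and stops its projectile movement.
; A looping timer then repeatedly launches the player toward the hook at timeline-driven speed, plus a push along the camera's forward vector.
; The hook destroys itself when the player overlaps its sphere.
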(event `self.ReceiveBeginPlay`
  (bind _ref_player (`self.REF_Player`)
    (:`then`
      (`CableComponent.SetAttachEndToComponent` (`self.Cable`) (`Character.Mesh` _ref_player) "head"))
    (:`else`)))

(event `self.Pro.OnComponentHit`
  (params (HitComponent :type "PrimitiveComponent Object Reference") (OtherActor :type "Actor Object Reference") (OtherComp :type "PrimitiveComponent Object Reference") (NormalImpulse :type "Vector Structure") (Hit :type "HitResult Structure (by ref)"))
  (`self.K2_AttachToActor` self OtherActor "None" "KeepWorld" "KeepWorld" "KeepWorld" true)
  (`ActorComponent.K2_DestroyComponent` (`self.ProjectileMovement`))
  (`self.REF_Player`
    (:`then`
      (`KismetSystemLibrary.K2_SetTimerDelegate` (delegate `RR`) 0.1 true)
      (bind (_direction _newtrack_0) (`Timeline|Timeline`)
        (:`Update`
          (set `self.Speed` _newtrack_0))))
    (:`else`)))

(event `RR`
  (`SceneComponent.K2_SetWorldRotation` (`self.Arrow`) (`KismetMathLibrary.FindLookAtRotation` (`self.K2_GetActorLocation` (`GameplayStatics.GetPlayerCharacter` 0)) (`SceneComponent.K2_GetComponentLocation` (`self.Pro`))) false false)
  (`Character.LaunchCharacter` (`self.REF_Player`) (+ (* (`SceneComponent.GetForwardVector` (`self.Arrow`)) (`KismetMathLibrary.Conv_DoubleToVector` (`self.Speed`))) (* (`SceneComponent.GetForwardVector` (`/Game/ThirdPerson/Blueprints/BP_ThirdPersonCharacter.FollowCamera` (`self.REF_Player`))) (`KismetMathLibrary.Conv_DoubleToVector` 300.0))) false false))

(event `self.Sphere.OnComponentBeginOverlap`
  (params (OverlappedComponent :type "PrimitiveComponent Object Reference") (OtherActor :type "Actor Object Reference") (OtherComp :type "PrimitiveComponent Object Reference") (OtherBodyIndex :type Integer) (bFromSweep :type Boolean) (SweepResult :type "HitResult Structure (by ref)"))
  (if (== (`self.REF_Player`) OtherActor)
    (`self.K2_DestroyActor`)))

(fn `UserConstructionScript`)